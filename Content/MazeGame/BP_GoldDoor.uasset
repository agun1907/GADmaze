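; BP_GoldDoor is a maze game door that opens in exchange for 150 of the player's gold.
; Interact checks PlayerGold on the cached MazeGamemode and either deducts the price or prints a warning.
; On payment, a Timeline lerps the mesh from StartLoc to EndLoc, then sets IsGoldOpened and calls GoldDoorOpened on the game mode.
; BeginPlay also caches a BP_GoldMan from player pawn 1, though nothing here uses it.
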(event EventBeginPlay
  (Utilities|FlowControl|Sequence
    (:then_0
      (bind _asmaze_gamemode (Utilities|Casting|CastToMazeGamemode (Game|GetGameMode)))
      (Variables|Default|SetAs%20Gamemode _asmaze_gamemode))
    (:then_1
      (bind _asbp_gold_man (Utilities|Casting|CastToBP_GoldMan (Game|Player|GetPlayerPawn 1))
        (:then
          (Variables|Default|SetAs%20BP%20Gold%20Man _asbp_gold_man))
        (:CastFailed
          (Development|PrintString "Hello"))))))

(event EventInteract
  (bind _as_gamemode (Variables|Default|GetAs%20Gamemode))
  (bind _as_gamemode_2 (Variables|Default|GetAs%20Gamemode))
  (if (>= (Variables|/Game/MazeGame/MazeGamemode.MazeGamemode_C|GetPlayerGold (Variables|Default|GetAs%20Gamemode)) 150)
    (Variables|/Game/MazeGame/MazeGamemode.MazeGamemode_C|SetPlayerGold _as_gamemode (- (Variables|/Game/MazeGame/MazeGamemode.MazeGamemode_C|GetPlayerGold _as_gamemode) 150))
    (bind _newtrack_0 (Timeline|Timeline Play)
      (:Update
        (Transformation|SetRelativeLocation (Variables|Default|GetStaticMesh) (Math|Vector|Lerp(Vector) (Variables|Default|GetStartLoc) (Variables|Default|GetEndLoc) _newtrack_0) false false))
      (:Finished
        (Variables|/Game/MazeGame/MazeGamemode.MazeGamemode_C|SetIsGoldOpened _as_gamemode_2 true)
        (Default|CallGoldDoorOpened _as_gamemode_2)))
    (else
      (Development|PrintString "You Need 150 gold to enter"))))

(fn ConstructionScript)