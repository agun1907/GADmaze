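; BP_EndDoor is the final door of the maze game, opening once the MazeGamemode's LastDoorOpened flag is set.
; Tick polls that flag and, through a DoOnce, plays a Timeline that lerps the mesh from StartLoc to EndLoc, then sets DoorOpened.
; While the flag is unset, first-person player overlap with the Box turns on the game mode's ShowEndBar; leaving clears it.
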(event OnComponentBeginOverlap(Box)
  (params (OverlappedComponent :type Primitive%20Component%20Object%20Reference) (OtherActor :type Actor%20Object%20Reference) (OtherComp :type Primitive%20Component%20Object%20Reference) (OtherBodyIndex :type Integer) (bFromSweep :type Boolean) (SweepResult :type Hit%20Result%20Structure%20%28by%20ref%29))
  (if (== OtherActor (Variables|Default|GetAs%20BP%20First%20Person%20Character))
    (if (not (Variables|/Game/MazeGame/MazeGamemode.MazeGamemode_C|GetLastDoorOpened (Variables|Default|GetAs%20Gamemode)))
      (Variables|/Game/MazeGame/MazeGamemode.MazeGamemode_C|SetShowEndBar (Variables|Default|GetAs%20Gamemode) true))))

(event OnComponentEndOverlap(Box)
  (params (OverlappedComponent :type Primitive%20Component%20Object%20Reference) (OtherActor :type Actor%20Object%20Reference) (OtherComp :type Primitive%20Component%20Object%20Reference) (OtherBodyIndex :type Integer))
  (if (== OtherActor (Variables|Default|GetAs%20BP%20First%20Person%20Character))
    (Variables|/Game/MazeGame/MazeGamemode.MazeGamemode_C|SetShowEndBar (Variables|Default|GetAs%20Gamemode) false)))

(event EventBeginPlay
  (Utilities|FlowControl|Sequence
    (:then_0
      (bind _asmaze_gamemode (Utilities|Casting|CastToMazeGamemode (Game|GetGameMode)))
      (Variables|Default|SetAs%20Gamemode _asmaze_gamemode))
    (:then_1
      (bind _asbp_gold_man (Utilities|Casting|CastToBP_GoldMan (Game|Player|GetPlayerPawn 1))
        (:then
          (Variables|Default|SetAs%20BP%20Gold%20Man _asbp_gold_man))
        (:CastFailed
          (Development|PrintString "Hello"))))
    (:then_2
      (bind _asbp_first_person_character (Utilities|Casting|CastToBP_FirstPersonCharacter (Game|GetPlayerCharacter 0)))
      (Variables|Default|SetAs%20BP%20First%20Person%20Character _asbp_first_person_character))))

(event EventTick
  (params (DeltaSeconds :type Float%20%28single-precision%29))
  (if (Variables|/Game/MazeGame/MazeGamemode.MazeGamemode_C|GetLastDoorOpened (Variables|Default|GetAs%20Gamemode))
    (Utilities|FlowControl|DoOnce false
      (:Completed
        (bind _newtrack_0 (Timeline|Timeline Play)
          (:Update
            (Transformation|SetRelativeLocation (Variables|Default|GetStaticMesh) (Math|Vector|Lerp(Vector) (Variables|Default|GetStartLoc) (Variables|Default|GetEndLoc) _newtrack_0) false false))
          (:Finished
            (Variables|Default|SetDoorOpened true)))))))

(fn ConstructionScript)