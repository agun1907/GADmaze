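; BP_MazeCell is a single maze cell that builds its floor and optional walls in the construction script.
; It derives wall thickness from GridSize, scales the floor, then adds scaled cube meshes for each enabled North, South, East or West wall.
; The Ceiling flag adds no mesh, only a downward-facing directional light near the wall top, with configurable intensity.
; The event graph holds no active logic.
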(event EventBeginPlay)

(event Collision|EventActorBeginOverlap
  (params (OtherActor :type Actor%20Object%20Reference)))

(event EventTick
  (params (DeltaSeconds :type Float%20%28single-precision%29)))

(fn ConstructionScript
  (bind _gridsize (Variables|Default|GetGridSize))
  (bind _gridsize_2 (Variables|Default|GetGridSize))
  (bind _returnvalue (* _gridsize_2 0.5))
  (bind _returnvalue_2 (/ _gridsize 1e+02))
  (Utilities|FlowControl|Sequence
    (:then_0
      (Variables|Default|SetWallTickness (/ (Variables|Default|GetGridSize) 1e+01)))
    (:then_1
      (Utilities|FlowControl|Sequence
        (:then_0
          (Transformation|SetRelativeScale3D (Variables|Default|GetFloor) (Math|Vector|MakeVector _returnvalue_2 _returnvalue_2 (/ (Variables|Default|GetWallTickness) 1e+02))))
        (:then_1
          (if (Variables|Default|GetSouthWall)
            (bind _returnvalue_3 (AddComponent|AddStaticMeshComponent false (Math|Transform|MakeTransform (Math|Vector|MakeVector (* (Variables|Default|GetWallTickness) -1.0) 0.0 (Variables|Default|GetWallTickness)) "0, 0, 0" (Math|Vector|MakeVector (/ (Variables|Default|GetWallTickness) 1e+02) (/ (Variables|Default|GetGridSize) 1e+02) (/ (Variables|Default|GetWallHeight) 1e+02)))))
            (Components|StaticMesh|SetStaticMesh _returnvalue_3 "/Game/LevelPrototyping/Meshes/SM_Cube.SM_Cube")))
        (:then_2
          (if (Variables|Default|GetNorthWall)
            (bind _returnvalue_4 (AddComponent|AddStaticMeshComponent false (Math|Transform|MakeTransform (Math|Vector|MakeVector (Variables|Default|GetGridSize) 0.0 (Variables|Default|GetWallTickness)) "0, 0, 0" (Math|Vector|MakeVector (/ (Variables|Default|GetWallTickness) 1e+02) (/ (Variables|Default|GetGridSize) 1e+02) (/ (Variables|Default|GetWallHeight) 1e+02)))))
            (Components|StaticMesh|SetStaticMesh _returnvalue_4 "/Game/LevelPrototyping/Meshes/SM_Cube.SM_Cube")))
        (:then_3
          (if (Variables|Default|GetWestWall)
            (bind _returnvalue_5 (AddComponent|AddStaticMeshComponent false (Math|Transform|MakeTransform (Math|Vector|MakeVector 0.0 0.0 (Variables|Default|GetWallTickness)) "0.000000,-90.000000,0.000000" (Math|Vector|MakeVector (/ (Variables|Default|GetWallTickness) 1e+02) (/ (Variables|Default|GetGridSize) 1e+02) (/ (Variables|Default|GetWallHeight) 1e+02)))))
            (Components|StaticMesh|SetStaticMesh _returnvalue_5 "/Game/LevelPrototyping/Meshes/SM_Cube.SM_Cube")))
        (:then_4
          (if (Variables|Default|GetEastWall)
            (bind _returnvalue_6 (AddComponent|AddStaticMeshComponent false (Math|Transform|MakeTransform (Math|Vector|MakeVector 0.0 (+ (Variables|Default|GetGridSize) (Variables|Default|GetWallTickness)) (Variables|Default|GetWallTickness)) "0.000000,-90.000000,0.000000" (Math|Vector|MakeVector (/ (Variables|Default|GetWallTickness) 1e+02) (/ (Variables|Default|GetGridSize) 1e+02) (/ (Variables|Default|GetWallHeight) 1e+02)))))
            (Components|StaticMesh|SetStaticMesh _returnvalue_6 "/Game/LevelPrototyping/Meshes/SM_Cube.SM_Cube")))
        (:then_5
          (if (Variables|Default|GetCeiling)
            (bind _returnvalue_7 (AddComponent|AddDirectionalLightComponent false (Math|Transform|MakeTransform (Math|Vector|MakeVector _returnvalue _returnvalue (- (Variables|Default|GetWallHeight) (Variables|Default|GetWallTickness))) (Math|Rotator|MakeRotator 0.0 -9e+01 0.0) "1.000000,1.000000,1.000000")))
            (Rendering|Components|Light|SetIntensity _returnvalue_7 (Variables|Default|GetLightIntensity))))))))