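; BP_Key is a key pickup for the maze game, identified by its KeyNumber.
; The construction script colors the mesh green for key 0 or red for key 1.
; On Interact, it writes KeyNumber to the cached MazeGamemode's Keys variable, replacing the previous value rather than accumulating keys.
; It then prints an acquired message using the matching KeyNames entry and destroys itself.
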(event EventBeginPlay
  (bind _asmaze_gamemode (Utilities|Casting|CastToMazeGamemode (Game|GetGameMode)))
  (Variables|Default|SetAs%20Gamemode _asmaze_gamemode))

(event EventInteract
  (bind _output_get (Variables|/Game/MazeGame/MazeGamemode.MazeGamemode_C|Setkeys (Variables|Default|GetAs%20Gamemode) (Variables|Default|GetKeyNumber)))
  (Development|PrintString (Utilities|String|Append "Key " (Utilities|Array|Get(acopy) (Variables|Default|GetKeyNames) _output_get) " Acquired"))
  (Actor|DestroyActor))

(fn ConstructionScript
  (bind _staticmesh (Variables|Default|GetStaticMesh))
  (switch int (Variables|Default|GetKeyNumber)
    (:0
      (Rendering|Material|SetMaterial _staticmesh 0 "/Game/MazeGame/greenmaterial.greenmaterial"))
    (:1
      (Rendering|Material|SetMaterial _staticmesh 0 "/Game/MazeGame/redmaterial.redmaterial"))))