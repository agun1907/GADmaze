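; BP_Door is an interactable locked door for the maze game that opens when the game mode's Keys value equals the door's KeyNumber.
; It caches MazeGamemode on BeginPlay, and on Interact a matching key plays a Timeline that lerps the mesh's relative location from StartLoc to EndLoc.
; A mismatch prints a wrong-key message.
; The construction script colors the mesh green or red according to KeyNumber.
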(event EventBeginPlay
  (bind _asmaze_gamemode (Utilities|Casting|CastToMazeGamemode (Game|GetGameMode)))
  (Variables|Default|SetAs%20Gamemode _asmaze_gamemode))

(event EventInteract
  (if (== (Variables|/Game/MazeGame/MazeGamemode.MazeGamemode_C|Getkeys (Variables|Default|GetAs%20Gamemode)) (Variables|Default|GetKeyNumber))
    (bind _newtrack_0 (Timeline|Timeline Play)
      (:Update
        (Transformation|SetRelativeLocation (Variables|Default|GetStaticMesh) (Math|Vector|Lerp(Vector) (Variables|Default|GetStartLoc) (Variables|Default|GetEndLoc) _newtrack_0) false false)))
    (else
      (Development|PrintString "You don't have the correct key"))))

(fn ConstructionScript
  (bind _staticmesh (Variables|Default|GetStaticMesh))
  (switch int (Variables|Default|GetKeyNumber)
    (:0
      (Rendering|Material|SetMaterial _staticmesh 0 "/Game/MazeGame/greenmaterial.greenmaterial"))
    (:1
      (Rendering|Material|SetMaterial _staticmesh 0 "/Game/MazeGame/redmaterial.redmaterial"))))