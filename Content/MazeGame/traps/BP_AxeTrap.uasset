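; Axe trap for the maze game that swings once the player enters its activation box and damages them on contact.
; The first player overlap destroys the activation box and plays a timeline that drives the axe's pitch rotation.
; Each player overlap with the damage box calls HealthUpdate on the cached first-person character to subtract health, independently of whether the axe has been triggered.
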(event OnComponentBeginOverlap(ActivisionBox)
  (params (OverlappedComponent :type Primitive%20Component%20Object%20Reference) (OtherActor :type Actor%20Object%20Reference) (OtherComp :type Primitive%20Component%20Object%20Reference) (OtherBodyIndex :type Integer) (bFromSweep :type Boolean) (SweepResult :type Hit%20Result%20Structure%20%28by%20ref%29))
  (if (== OtherActor (Variables|Default|GetAs%20BP%20First%20Person%20Character))
    (Components|DestroyComponent (Variables|Default|GetActivisionBox))
    (bind _newtrack_0 (Timeline|Axes Play)
      (:Update
        (Transformation|SetRelativeRotation (Variables|Default|GetAxe) (Math|Rotator|MakeRotator 0.0 (* _newtrack_0 3.6e+02) 0.0) false false)))))

(event OnComponentBeginOverlap(DamageBox)
  (params (OverlappedComponent :type Primitive%20Component%20Object%20Reference) (OtherActor :type Actor%20Object%20Reference) (OtherComp :type Primitive%20Component%20Object%20Reference) (OtherBodyIndex :type Integer) (bFromSweep :type Boolean) (SweepResult :type Hit%20Result%20Structure%20%28by%20ref%29))
  (bind _as_bp_first_person_character (Variables|Default|GetAs%20BP%20First%20Person%20Character))
  (if (== OtherActor _as_bp_first_person_character)
    (Default|HealthUpdate _as_bp_first_person_character -35.0)))

(event EventBeginPlay
  (bind _asbp_first_person_character (Utilities|Casting|CastToBP_FirstPersonCharacter (Game|GetPlayerCharacter 0)))
  (Variables|Default|SetAs%20BP%20First%20Person%20Character _asbp_first_person_character))

(fn ConstructionScript)