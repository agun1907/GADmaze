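; BP_TrapGas is a maze gas trap that deals damage over time while the first-person player is inside its DamageBOx volume.
; Overlap start runs a looping DOT timer that calls HealthUpdate on the player, and overlap end clears it.
; It binds to a trap event on the player character; when the event's trap type matches its own, the box's collision is disabled and the Gas component destroyed.
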(event OnComponentBeginOverlap(DamageBOx)
  (params (OverlappedComponent :type Primitive%20Component%20Object%20Reference) (OtherActor :type Actor%20Object%20Reference) (OtherComp :type Primitive%20Component%20Object%20Reference) (OtherBodyIndex :type Integer) (bFromSweep :type Boolean) (SweepResult :type Hit%20Result%20Structure%20%28by%20ref%29))
  (if (== OtherActor (Variables|Default|GetAs%20BP%20First%20Person%20Character))
    (Utilities|Time|SetTimerbyFunctionName 0 "DOT" (Variables|Default|GetDOTtime) true)))

(event OnComponentEndOverlap(DamageBOx)
  (params (OverlappedComponent :type Primitive%20Component%20Object%20Reference) (OtherActor :type Actor%20Object%20Reference) (OtherComp :type Primitive%20Component%20Object%20Reference) (OtherBodyIndex :type Integer))
  (if (== OtherActor (Variables|Default|GetAs%20BP%20First%20Person%20Character))
    (Utilities|Time|ClearTimerbyFunctionName 0 "DOT")))

(event Custom|CustomEvent
  (params (TrapTypes :type TrapTypes%20Enum :default "NewEnumerator0"))
  (if (Utilities|Enum|Equal(Enum) TrapTypes (Variables|Default|GetTrapType))
    (Collision|SetCollisionEnabled (Variables|Default|GetDamageBOx) "NoCollision")
    (Components|DestroyComponent (Variables|Default|GetGas))))

(event Custom|DOT
  (Default|HealthUpdate (Variables|Default|GetAs%20BP%20First%20Person%20Character) (Variables|Default|GetDOTDamage)))

(event EventBeginPlay
  (bind _asbp_first_person_character (Utilities|Casting|CastToBP_FirstPersonCharacter (Game|GetPlayerCharacter 0)))
  (bind _output_get (Variables|Default|SetAs%20BP%20First%20Person%20Character _asbp_first_person_character))
  (EventDispatchers|BindEventtoDPTrap _output_get (delegate Custom|CustomEvent)))

(fn ConstructionScript)