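; BP_Spike is a maze trap whose spikes move when the player's first-person character enters the Activision trigger.
; That overlap plays a timeline, which on each update adds the scaled track value to the spikes' current relative Z, so the offset accumulates.
; A separate DamageBOx overlap applies fixed damage through the character's HealthUpdate.
; Both overlaps respond only to the player character cached at BeginPlay.
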(event OnComponentBeginOverlap(Activision)
  (params (OverlappedComponent :type Primitive%20Component%20Object%20Reference) (OtherActor :type Actor%20Object%20Reference) (OtherComp :type Primitive%20Component%20Object%20Reference) (OtherBodyIndex :type Integer) (bFromSweep :type Boolean) (SweepResult :type Hit%20Result%20Structure%20%28by%20ref%29))
  (bind _spikes (Variables|Default|GetSpikes))
  (bind _relativelocation (Variables|/Script/Engine.SceneComponent|GetRelativeLocation _spikes))
  (if (== OtherActor (Variables|Default|GetAs%20BP%20First%20Person%20Character))
    (bind _newtrack_0 (Timeline|Timeline Play)
      (:Update
        (Transformation|SetRelativeLocation _spikes (Math|Vector|MakeVector (.x _relativelocation) (.y _relativelocation) (+ (.z _relativelocation) (* _newtrack_0 15.0))) false false)))))

(event OnComponentBeginOverlap(DamageBOx)
  (params (OverlappedComponent :type Primitive%20Component%20Object%20Reference) (OtherActor :type Actor%20Object%20Reference) (OtherComp :type Primitive%20Component%20Object%20Reference) (OtherBodyIndex :type Integer) (bFromSweep :type Boolean) (SweepResult :type Hit%20Result%20Structure%20%28by%20ref%29))
  (bind _as_bp_first_person_character (Variables|Default|GetAs%20BP%20First%20Person%20Character))
  (if (== OtherActor _as_bp_first_person_character)
    (Default|HealthUpdate _as_bp_first_person_character -15.0)))

(event EventBeginPlay
  (bind _asbp_first_person_character (Utilities|Casting|CastToBP_FirstPersonCharacter (Game|GetPlayerCharacter 0)))
  (Variables|Default|SetAs%20BP%20First%20Person%20Character _asbp_first_person_character))

(fn ConstructionScript)